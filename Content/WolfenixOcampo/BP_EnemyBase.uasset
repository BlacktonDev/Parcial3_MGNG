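; BP_EnemyBase is an enemy Blueprint that handles health, damage intake and death.
; The construction script seeds current health and damage from their maximums, and BeginPlay caches a reference to the player.
; AnyDamage lowers health with a floor at zero.
; At zero it sets IsDead, jumps the anim instance to the death node, disables capsule collision, detaches the controller, and destroys the actor after a short delay.
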(event EventBeginPlay
  (bind _asbp_player (Utilities|Casting|CastToBP_Player (Game|GetPlayerCharacter 0)))
  (Variables|Default|SetPlayer%20Ref _asbp_player))

(event Game|Damage|EventAnyDamage
  (params (Damage :type Float%20%28single-precision%29) (DamageType :type Damage%20Type%20Object%20Reference) (InstigatedBy :type Controller%20Object%20Reference) (DamageCauser :type Actor%20Object%20Reference))
  (bind _output_get (Variables|Default|SetCurrent%20Health (Math|Float|Clamp(Float) (- (Variables|Default|GetCurrent%20Health) Damage) 0.0 (- (Variables|Default|GetCurrent%20Health) Damage))))
  (if (== _output_get 0.0)
    (Variables|Default|SetIsDead true)
    (if (Variables|Default|GetIsDead)
      (Class|PaperZDAnimInstance|JumptoNode (Class|PaperZDCharacter|GetAnimInstance) (Variables|Default|GetDeadAnimName) "None")
      (Collision|SetCollisionEnabled (Variables|Default|GetCapsuleComponent) "NoCollision")
      (Class|Pawn|DetachfromControllerPendingDestroy)
      (Utilities|FlowControl|Delay 1.0)
      (Actor|DestroyActor))))

(fn ConstructionScript
  (Variables|Default|SetCurrent%20Health (Variables|Default|GetMax%20Health))
  (Variables|Default|SetCurrent%20Damage (Variables|Default|GetMax%20Damage)))