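; BP_Enemy is an AI-driven sprite enemy that takes damage, dies and attacks the player.
; Damage lowers clamped health, then either shows a widget message with a timed pain state or triggers defeat and delayed destruction, syncing Busy and IsDead to the blackboard.
; A sphere overlap replays the attack animation every second while the player stays in range.
; That loop deals no damage; MakeDamage applies it separately and is not called here.
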(event OnComponentBeginOverlap(Sphere)
  (params (OverlappedComponent :type Primitive%20Component%20Object%20Reference) (OtherActor :type Actor%20Object%20Reference) (OtherComp :type Primitive%20Component%20Object%20Reference) (OtherBodyIndex :type Integer) (bFromSweep :type Boolean) (SweepResult :type Hit%20Result%20Structure%20%28by%20ref%29))
  (bind _output_get (Variables|Default|SetPlayerInRange true))
  (if (and _output_get (Components|ComponentHasTag OtherComp "Player")) :!label _label
    (Variables|Default|SetIsBusy true)
    (Class|PaperZDAnimInstance|JumptoNode (Class|PaperZDCharacter|GetAnimInstance) "JumpAttack" "None")
    (Utilities|FlowControl|Delay 1.0)
    (goto _label)))

(event OnComponentEndOverlap(Sphere)
  (params (OverlappedComponent :type Primitive%20Component%20Object%20Reference) (OtherActor :type Actor%20Object%20Reference) (OtherComp :type Primitive%20Component%20Object%20Reference) (OtherBodyIndex :type Integer))
  (Variables|Default|SetPlayerInRange false))

(event EventBeginPlay
  (Variables|/Script/Engine.CharacterMovementComponent|SetMaxWalkSpeed (Variables|Character|GetCharacterMovement) (* (Variables|Default|GetSpeed) 1e+02))
  (Variables|Default|SetCurrentHealth (Variables|Default|GetMaxHealth)))

(event Collision|EventActorBeginOverlap
  (params (OtherActor :type Actor%20Object%20Reference)))

(event EventTick
  (params (DeltaSeconds :type Float%20%28single-precision%29)))

(event Game|Damage|EventAnyDamage
  (params (Damage :type Float%20%28single-precision%29) (DamageType :type Damage%20Type%20Object%20Reference) (InstigatedBy :type Controller%20Object%20Reference) (DamageCauser :type Actor%20Object%20Reference))
  (bind _output_get (Variables|Default|SetCurrentHealth (Math|Float|Clamp(Float) (- (Variables|Default|GetCurrentHealth) Damage) 0.0 (Variables|Default|GetMaxHealth))))
  (if (<= _output_get 0.0)
    (bind _output_get_2 (Variables|Default|SetIsDead true))
    (AI|Components|Blackboard|SetValueasBool (AI|GetBlackboard 0) (Utilities|Name|MakeLiteralName "IsDead") _output_get_2)
    (Collision|SetCollisionEnabled (Variables|Default|GetCapsuleComponent) "NoCollision")
    (Class|PaperZDAnimInstance|JumptoNode (Class|PaperZDCharacter|GetAnimInstance) "JumpDefeated" "None")
    (Utilities|FlowControl|Delay 5.0)
    (Actor|DestroyActor)
    (else
      (Class|BPIHealthWidget|UpdateDamage(Message) (UserInterface|GetWidget (Variables|Default|GetWidget)) (Utilities|Text|ToText(Float) Damage "HalfToEven") false)
      (bind _output_get_3 (Variables|Default|SetIsBusy true))
      (AI|Components|Blackboard|SetValueasBool (AI|GetBlackboard 0) (Utilities|Name|MakeLiteralName "Busy") _output_get_3)
      (Class|PaperZDAnimInstance|JumptoNode (Class|PaperZDCharacter|GetAnimInstance) "JumpPain" "None")
      (Utilities|FlowControl|Delay 1.0)
      (bind _output_get_4 (Variables|Default|SetIsBusy false))
      (AI|Components|Blackboard|SetValueasBool (AI|GetBlackboard 0) (Utilities|Name|MakeLiteralName "Busy") _output_get_4))))

(event EventUpdateDamage
  (params (Damage :type Text) (isHealing :type Boolean)))

(fn ConstructionScript)

(fn MakeDamage
  (params (OtherObject :type Object%20Object%20Reference) (IsOverlapping :type Boolean))
  (bind _returnvalue (Game|GetPlayerCharacter 0))
  (if IsOverlapping
    (if (== OtherObject _returnvalue)
      (Game|Damage|ApplyDamage _returnvalue (Variables|Default|GetDamage) 0 self))))