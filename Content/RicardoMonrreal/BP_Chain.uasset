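; BP_Chain builds a breakable physics chain from static mesh links when play begins.
; A loop adds NumberChains mesh components spaced along local Y, each mass-overridden and constrained to the XZ plane.
; Physics constraints join neighboring links with limited Swing1, locked Swing2 and twist, and a linear break threshold derived from BreakableForceLimit.
; Only intermediate links simulate physics, leaving both ends as fixed anchors.
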(event EventBeginPlay
  (bind _chainarray (Variables|Default|GetChainArray))
  (bind _chainarray_2 (Variables|Default|GetChainArray))
  (bind _returnvalue (Utilities|Array|LastIndex _chainarray))
  (bind _output (Utilities|Array|Get(acopy) _chainarray _returnvalue))
  (for _index (range 1 (Variables|Default|GetNumberChains))
    (Variables|Default|SetActualIndex _index)
    ;[1 1 1] Create Chain Mesh
    (bind _returnvalue_2 (Game|AddComponentbyClass "/Script/Engine.StaticMeshComponent" false))
    (Components|StaticMesh|SetStaticMesh _returnvalue_2 "/Game/RicardoMonrreal/chain.chain")
    (Class|PrimitiveComponent|SetConstraintMode _returnvalue_2 "XZPlane")
    (Class|PrimitiveComponent|SetMassOverrideinKg _returnvalue_2 "None" 1e+01 true)
    ;[1 1 1] Add to array
    (Utilities|Array|Add (Variables|Default|GetChainArray) _returnvalue_2)
    (Transformation|SetRelativeTransform (Utilities|Array|Get(acopy) _chainarray_2 (Utilities|Array|LastIndex _chainarray_2)) (Math|Transform|MakeTransform (Math|Vector|MakeVector 0.0 (- (Variables|Default|GetMeshPos) 25.0) 0.0) (Math|Rotator|MakeRotator 0.0 0.0 0.0) "1.000000,1.000000,1.000000") false false)
    (bind _output_get (Variables|Default|SetMeshPos (- (Variables|Default|GetMeshPos) 25.0)))
    (if (> (Variables|Default|GetActualIndex) 1)
      (bind _returnvalue_3 (Game|AddComponentbyClass "/Script/Engine.PhysicsConstraintComponent" false (Math|Transform|MakeTransform (Math|Vector|MakeVector 0.0 (+ _output_get 15.0) 0.0) "0, 0, 0" "1.000000,1.000000,1.000000")))
      (Class|PhysicsConstraintComponent|SetLinearBreakable _returnvalue_3 true (Class|KismetMathLibrary|Exp (Variables|Default|GetBreakableForceLimit)))
      (Class|PhysicsConstraintComponent|SetDisableCollision _returnvalue_3 true)
      (Class|PhysicsConstraintComponent|SetConstrainedComponents _returnvalue_3 (Utilities|Array|Get(acopy) _chainarray (- _returnvalue 1)) "None" _output "None")
      (Class|PhysicsConstraintComponent|SetAngularSwing1Limit _returnvalue_3 "ACM_Limited" 45.0)
      (Class|PhysicsConstraintComponent|SetAngularSwing2Limit _returnvalue_3 "ACM_Locked" 0.0)
      (Class|PhysicsConstraintComponent|SetAngularTwistLimit _returnvalue_3 "ACM_Locked" 0.0)
      (if (and (!= (Variables|Default|GetActualIndex) (Variables|Default|GetNumberChains)) (!= (Variables|Default|GetActualIndex) 1))
        (Physics|SetSimulatePhysics _output true)))))

(event Collision|EventActorBeginOverlap
  (params (OtherActor :type Actor%20Object%20Reference)))

(event EventTick
  (params (DeltaSeconds :type Float%20%28single-precision%29)))

(fn ConstructionScript)