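; BP_healBox is a healing volume that periodically heals an overlapping actor tagged "Healable".
; Begin overlap on HealBox sets an Overlap flag and starts a Delay loop that sends HealActorMessage with HealValue every HealingInterval.
; End overlap clears that single flag, which is shared by all overlapping actors, so the loop stops at its next check.
; SetDamage is an empty stub.
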(event OnComponentBeginOverlap(HealBox)
  (params (OverlappedComponent :type Primitive%20Component%20Object%20Reference) (OtherActor :type Actor%20Object%20Reference) (OtherComp :type Primitive%20Component%20Object%20Reference) (OtherBodyIndex :type Integer) (bFromSweep :type Boolean) (SweepResult :type Hit%20Result%20Structure%20%28by%20ref%29))
  ;[0 1 0] Comprueba que el tag del objeto overlapeado e incrementa la vida del objeto
  (bind _output_get (Variables|Default|SetOverlap true))
  (if (and _output_get (Actor|ActorHasTag OtherActor "Healable")) :!label _label
    (Class|BPIHeal|HealActor(Message) OtherActor (Variables|Default|GetHealValue))
    (Utilities|FlowControl|Delay (Variables|Default|GetHealingInterval))
    (goto _label)))

(event OnComponentEndOverlap(HealBox)
  (params (OverlappedComponent :type Primitive%20Component%20Object%20Reference) (OtherActor :type Actor%20Object%20Reference) (OtherComp :type Primitive%20Component%20Object%20Reference) (OtherBodyIndex :type Integer))
  (Variables|Default|SetOverlap false))

(event EventBeginPlay)

(event Collision|EventActorBeginOverlap
  (params (OtherActor :type Actor%20Object%20Reference)))

(event EventTick
  (params (DeltaSeconds :type Float%20%28single-precision%29)))

(fn ConstructionScript)

(fn SetDamage
  (params (Damage :type Text) (SelfWidget :type Object%20Object%20Reference))
  (return 0))