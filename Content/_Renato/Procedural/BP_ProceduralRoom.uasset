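; Procedural room or corridor builder that tiles floors, walls and roofs as mesh instances at construction and BeginPlay.
; SeparatelyInstancedRooms drives the layout, with BasicRoom an uncalled variant.
; Side walls get doors by manual rules or seeded streams whose odds fall as doors spawn, and steps randomly replace upper floor tiles.
; Each indexed side wall spawns a BP_WallCollision, and DeleteWall removes an instance, moving the last collision entry into its index.
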(event Custom|DeleteWall
  (params (Index :type Integer))
  (bind _wallcollisions (Variables|Default|GetWallCollisions))
  (bind _returnvalue (Utilities|Array|LastIndex _wallcollisions))
  (bind _output (Utilities|Array|Get(acopy) _wallcollisions _returnvalue))
  ;[0 0.5392 1] Remove wall instance at provided index
  (Class|InstancedStaticMeshComponent|RemoveInstance (Variables|Default|GetIndexedWall) Index)
  ;[0 0.5962 1] Update collisions to match wall instance array
  (Utilities|Array|SetArrayElem _wallcollisions Index _output true)
  (Default|Update _output Index)
  (Utilities|Array|RemoveIndex (Variables|Default|GetWallCollisions) _returnvalue))

(event EventBeginPlay
  (CallFunction|SeparatelyInstancedRooms))

(fn ConstructionScript
  (Utilities|Array|Clear (Variables|Default|GetDoors))
  (Utilities|Array|Clear (Variables|Default|GetSteps))
  (CallFunction|SeparatelyInstancedRooms))

(fn BasicRoom
  ;[0 0.5009 1] CreateFloor
  (for _index (range 0 (- (Variables|Default|GetRoomTilesX) 1))
    (Components|InstancedStaticMesh|AddInstance (Variables|Default|GetFloor) (Math|Transform|MakeTransform (Math|Vector|MakeVector (* _index (Variables|Default|GetTileSizeX)) 0.0 0.0) "0, 0, 0" "1.000000,1.000000,1.000000") false)
    ;[0 0.6042 1] Bottom Tile
    (if (Variables|Default|GetIsBottomTile)
      (Components|InstancedStaticMesh|AddInstance (Variables|Default|GetFloor) (Math|Transform|MakeTransform (Math|Vector|MakeVector (* (Variables|Default|GetTileSizeX) (+ _index 1)) 4e+02 0.0) "-180.000000,0.000000,-90.000000" "1.000000,1.000000,1.000000") false)))
  ;[0 0.6499 1] Checks
  (if (> (Variables|Default|GetWallTileX) (Variables|Default|GetRoomTilesX))
    ;[0 0.5689 1] Y height manager
    (for _index_2 (range 0 (- (Variables|Default|GetWallTileX) 1))
      (Components|InstancedStaticMesh|AddInstance (Variables|Default|GetWall) (Math|Transform|MakeTransform (Math|Vector|MakeVector 0.0 0.0 (* (Variables|Default|GetWallSizeX) _index_2)) "0, 0, 0" "1.000000,1.000000,1.000000") false)
      (for _index_3 (range 1 (- (Variables|Default|GetRoomTilesX) 1))
        (Components|InstancedStaticMesh|AddInstance (Variables|Default|GetWall) (Math|Transform|MakeTransform (Math|Vector|MakeVector (* _index_3 (Variables|Default|GetTileSizeX)) 0.0 (* (Variables|Default|GetWallSizeX) _index_2)) "0, 0, 0" "1.000000,1.000000,1.000000") false)))
    (else
      ;[0 0.427 1] Background walls
      (for _index_4 (range 2 (- (Variables|Default|GetWallTileX) 1))
        (Components|InstancedStaticMesh|AddInstance (Variables|Default|GetWall) (Math|Transform|MakeTransform (Math|Vector|MakeVector (* (Variables|Default|GetWallSizeX) _index_4) 0.0 0.0) "0, 0, 0" "1.000000,1.000000,1.000000") false)
        ;[0 0.5825 1] Roof
        (if (and (Variables|Default|GetHasRoof) (Variables|Default|GetIsCorridor))
          (Components|InstancedStaticMesh|AddInstance (Variables|Default|GetFloor) (Math|Transform|MakeTransform (Math|Vector|MakeVector (* (Variables|Default|GetTileSizeX) (+ _index_4 1)) 0.0 4e+02) "180.000000,0.000000,0.000000" "1.000000,1.000000,1.000000") false)))
      ;[0 0.5608 1] Set wall height
      (for _index_5 (range 0 (- (Variables|Default|GetWallTileX) 1))
        (Components|InstancedStaticMesh|AddInstance (Variables|Default|GetWall) (Math|Transform|MakeTransform (Math|Vector|MakeVector 0.0 0.0 (* _index_5 (Variables|Default|GetWallSizeX))) "0, 0, 0" "1.000000,1.000000,1.000000") false)
        (for _index_6 (range 1 (- (Variables|Default|GetRoomTilesX) 1))
          (Components|InstancedStaticMesh|AddInstance (Variables|Default|GetWall) (Math|Transform|MakeTransform (Math|Vector|MakeVector (* (Variables|Default|GetWallSizeX) _index_6) 0.0 (* _index_5 (Variables|Default|GetWallSizeX))) "0, 0, 0" "1.000000,1.000000,1.000000") false)))))
  ;[0 0.6644 1] Steps
  (if (Variables|Default|GetHasSteps)
    (for _index_7 (range 1 (- (Variables|Default|GetWallTileX) 1))
      ;[0 0.5316 1] Steps entry check
      (if (or (Variables|Default|GetIsOriginRoom) (!= _index_7 0))
        (CallFunction|SteporFloor (== (Math|Integer|%(Integer) _index_7 (Variables|Default|GetStepDoorEvery)) (Variables|Default|GetStepDoorRemainder)) (Math|Vector|MakeVector 0.0 0.0 (* _index_7 (Variables|Default|GetWallSizeX))) "0, 0, 0"))
      (for _index_8 (range 0 (- (Variables|Default|GetRoomTilesX) 1))
        (CallFunction|SteporFloor (== (Math|Integer|%(Integer) _index_8 (Variables|Default|GetStepDoorEvery)) (Variables|Default|GetStepDoorRemainder)) (Math|Vector|MakeVector (* _index_8 (Variables|Default|GetTileSizeX)) 0.0 (* _index_7 (Variables|Default|GetWallSizeX))) "0, 0, 0"))))
  ;[0 0.5179 1] Roof handler
  (if (Variables|Default|GetHasRoof)
    (for _index_9 (range 0 (- (Variables|Default|GetRoomTilesX) 1))
      (Components|InstancedStaticMesh|AddInstance (Variables|Default|GetFloor) (Math|Transform|MakeTransform (Math|Vector|MakeVector (* (Variables|Default|GetTileSizeX) _index_9) 0.0 (* (Variables|Default|GetTileSizeX) (Variables|Default|GetWallTileX))) "0, 0, 0" "1.000000,1.000000,1.000000") false)))
  ;[0 0.6304 1] Handle Left wall height
  (for _index_10 (range 0 (- (Variables|Default|GetWallTileX) 1))
    ;[0 0.5139 1] Entry check
    (if (or (Variables|Default|GetIsOriginRoom) (!= _index_10 0))
      (CallFunction|WallorDoorL (== (Math|Integer|%(Integer) _index_10 (Variables|Default|GetDoorEvery)) (Variables|Default|GetDoorRemainder)) (Math|Vector|MakeVector 0.0 0.0 (* _index_10 (Variables|Default|GetWallSizeX))) "0.000000,90.000000,0.000000"))
    ;[0 0.6006 1] Handle Right wall Height
    (CallFunction|WallorDoorL (== (Math|Integer|%(Integer) _index_10 (Variables|Default|GetDoorEvery)) (Variables|Default|GetDoorRemainder)) (Math|Vector|MakeVector (* (Variables|Default|GetRoomTilesX) (Variables|Default|GetTileSizeX)) 0.0 (* _index_10 (Variables|Default|GetWallSizeX))) "0.000000,90.000000,0.000000")))

(fn WallorDoorL
  (params (CanDoor :type Boolean) (InstanceTransformLocation :type Vector) (InstanceTransformRotation :type Rotator))
  (bind _returnvalue (Transformation|GetActorTransform))
  (bind _leftdoorcount (Variables|Default|GetLeftDoorCount))
  (bind _returnvalue_2 (Math|Transform|TransformLocation _returnvalue InstanceTransformLocation))
  (bind _returnvalue_3 (Math|Transform|TransformRotation _returnvalue InstanceTransformRotation))
  ;[0 0.5622 1] Is this a door
  (if (and CanDoor (Class|KismetMathLibrary|RandomBoolwithWeightfromStream (Variables|Default|GetRoomStream) (/ (- _leftdoorcount (Utilities|Array|Length (Variables|Default|GetDoors))) _leftdoorcount)))
    ;[0 0.4894 1] Transform location and rotation to world space, spawn door and add to array
    (bind _returnvalue_4 (Game|SpawnActorfromClass "/Game/_Renato/Procedural/SpawnedObjects/BP_Doors.BP_Doors_C" (Math|Transform|MakeTransform _returnvalue_2 _returnvalue_3 "1.000000,1.000000,1.000000") "Undefined" "MultiplyWithRoot" 0 true 0))
    (Utilities|Array|Add (Variables|Default|GetDoors) _returnvalue_4)
    (Utilities|Array|SetArrayElem (Variables|/Script/Engine.Actor|GetTags _returnvalue_4) 0 "InstancedDoor")
    (else
      ;[0 0.5514 1] Add wall instead
      (bind _returnvalue_5 (Components|InstancedStaticMesh|AddInstance (Variables|Default|GetIndexedWall) (Math|Transform|MakeTransform InstanceTransformLocation InstanceTransformRotation "1.000000,1.000000,1.000000") false))
      ;[0 0.4466 1] Add colliders to walls
      (bind _returnvalue_6 (Game|SpawnActorfromClass "/Game/_Renato/Procedural/BP_WallCollision.BP_WallCollision_C" (Math|Transform|MakeTransform _returnvalue_2 _returnvalue_3 "1.000000,1.000000,1.000000") "Undefined" "MultiplyWithRoot" 0 _returnvalue_5 0))
      (Utilities|Array|Add (Variables|Default|GetWallCollisions) _returnvalue_6))))

(fn SteporFloor
  (params (CanVault :type Boolean) (InstanceTransformLocation :type Vector) (InstanceTransformRotation :type Rotator))
  (bind _returnvalue (Transformation|GetActorTransform))
  (bind _stepdoorcount (Variables|Default|GetStepDoorCount))
  ;[0 0.5622 1] Is this a vault
  (if (and CanVault (Class|KismetMathLibrary|RandomBoolwithWeightfromStream (Variables|Default|GetStepStream) (/ (- _stepdoorcount (Utilities|Array|Length (Variables|Default|GetSteps))) _stepdoorcount)))
    ;[0 0.4894 1] Transform location and rotation to world space, spawn door and add to array
    (bind _returnvalue_2 (Game|SpawnActorfromClass "/Game/_Renato/Procedural/SpawnedObjects/BP_Steps.BP_Steps_C" (Math|Transform|MakeTransform (Math|Transform|TransformLocation _returnvalue InstanceTransformLocation) (Math|Transform|TransformRotation _returnvalue InstanceTransformRotation) "1.000000,1.000000,1.000000") "Undefined" "MultiplyWithRoot" 0 0))
    (Utilities|Array|Add (Variables|Default|GetSteps) _returnvalue_2)
    (else
      ;[0 0.5514 1] Add floor instead
      (Components|InstancedStaticMesh|AddInstance (Variables|Default|GetFloor) (Math|Transform|MakeTransform InstanceTransformLocation InstanceTransformRotation "1.000000,1.000000,1.000000") false))))

(fn SeparatelyInstancedRooms
  (bind _tilesizex (Variables|Default|GetTileSizeX))
  ;[0 0.5009 1] CreateFloor
  (for _index (range 0 (- (Variables|Default|GetRoomTilesX) 1))
    (Components|InstancedStaticMesh|AddInstance (Variables|Default|GetFloor) (Math|Transform|MakeTransform (Math|Vector|MakeVector (* _index (Variables|Default|GetTileSizeX)) 0.0 0.0) "0, 0, 0" "1.000000,1.000000,1.000000") false)
    ;[0 0.6042 1] Bottom Tile
    (if (Variables|Default|GetIsBottomTile)
      (Components|InstancedStaticMesh|AddInstance (Variables|Default|GetFloor) (Math|Transform|MakeTransform (Math|Vector|MakeVector (* (Variables|Default|GetTileSizeX) (+ _index 1)) 4e+02 0.0) "-180.000000,0.000000,-90.000000" "1.000000,1.000000,1.000000") false)))
  (if (Variables|Default|GetIsCorridor)
    ;[0 0.5539 1] Hallway height
    (for _index_2 (range 0 (- (Variables|Default|GetWallTileX) 1))
      (Components|InstancedStaticMesh|AddInstance (Variables|Default|GetWall) (Math|Transform|MakeTransform (Math|Vector|MakeVector (* (Variables|Default|GetWallSizeX) _index_2) 0.0 0.0) "0, 0, 0" "1.000000,1.000000,1.000000") false)
      ;[0 0.5825 1] Handle corridor roof
      (if (and (Variables|Default|GetHasRoof) (Variables|Default|GetIsCorridor))
        (Components|InstancedStaticMesh|AddInstance (Variables|Default|GetFloor) (Math|Transform|MakeTransform (Math|Vector|MakeVector (* (Variables|Default|GetTileSizeX) _index_2) 0.0 (* (Variables|Default|GetTileSizeX) 1.0)) "0, 0, 0" "1.000000,1.000000,1.000000") false)))
    (else
      ;[0 0.6499 1] Checks
      (if (> (Variables|Default|GetWallTileX) (Variables|Default|GetRoomTilesX))
        ;[0 0.5689 1] Y height manager
        (for _index_3 (range 0 (- (Variables|Default|GetWallTileX) 1))
          (Components|InstancedStaticMesh|AddInstance (Variables|Default|GetWall) (Math|Transform|MakeTransform (Math|Vector|MakeVector 0.0 0.0 (* (Variables|Default|GetWallSizeX) _index_3)) "0, 0, 0" "1.000000,1.000000,1.000000") false)
          (for _index_4 (range 1 (- (Variables|Default|GetRoomTilesX) 1))
            (Components|InstancedStaticMesh|AddInstance (Variables|Default|GetWall) (Math|Transform|MakeTransform (Math|Vector|MakeVector (* _index_4 (Variables|Default|GetTileSizeX)) 0.0 (* (Variables|Default|GetWallSizeX) _index_3)) "0, 0, 0" "1.000000,1.000000,1.000000") false)))
        (else
          ;[0 0.427 1] Background walls
          (for _index_5 (range 2 (- (Variables|Default|GetWallTileX) 1))
            (Components|InstancedStaticMesh|AddInstance (Variables|Default|GetWall) (Math|Transform|MakeTransform (Math|Vector|MakeVector (* (Variables|Default|GetWallSizeX) _index_5) 0.0 0.0) "0, 0, 0" "1.000000,1.000000,1.000000") false))
          ;[0 0.5608 1] Set wall height
          (for _index_6 (range 0 (- (Variables|Default|GetWallTileX) 1))
            (Components|InstancedStaticMesh|AddInstance (Variables|Default|GetWall) (Math|Transform|MakeTransform (Math|Vector|MakeVector 0.0 0.0 (* _index_6 (Variables|Default|GetWallSizeX))) "0, 0, 0" "1.000000,1.000000,1.000000") false)
            (for _index_7 (range 1 (- (Variables|Default|GetRoomTilesX) 1))
              (Components|InstancedStaticMesh|AddInstance (Variables|Default|GetWall) (Math|Transform|MakeTransform (Math|Vector|MakeVector (* (Variables|Default|GetWallSizeX) _index_7) 0.0 (* _index_6 (Variables|Default|GetWallSizeX))) "0, 0, 0" "1.000000,1.000000,1.000000") false)))))
      ;[0 0.6644 1] Steps
      (if (Variables|Default|GetHasSteps)
        (for _index_8 (range 1 (- (Variables|Default|GetWallTileX) 1))
          ;[0 0.5316 1] Steps entry check
          (if (or (Variables|Default|GetIsOriginRoom) (!= _index_8 0))
            (CallFunction|SteporFloor (== (Math|Integer|%(Integer) _index_8 (Variables|Default|GetStepDoorEvery)) (Variables|Default|GetStepDoorRemainder)) (Math|Vector|MakeVector 0.0 0.0 (* _index_8 (Variables|Default|GetWallSizeX))) "0, 0, 0"))
          (for _index_9 (range 0 (- (Variables|Default|GetRoomTilesX) 1))
            (CallFunction|SteporFloor (== (Math|Integer|%(Integer) _index_9 (Variables|Default|GetStepDoorEvery)) (Variables|Default|GetStepDoorRemainder)) (Math|Vector|MakeVector (* _index_9 (Variables|Default|GetTileSizeX)) 0.0 (* _index_8 (Variables|Default|GetWallSizeX))) "0, 0, 0"))))
      ;[0 0.5179 1] Roof handler
      (if (Variables|Default|GetHasRoof)
        (for _index_10 (range 0 (- (Variables|Default|GetRoomTilesX) 1))
          (Components|InstancedStaticMesh|AddInstance (Variables|Default|GetFloor) (Math|Transform|MakeTransform (Math|Vector|MakeVector (* (Variables|Default|GetTileSizeX) _index_10) 0.0 (* (Variables|Default|GetTileSizeX) (Variables|Default|GetWallTileX))) "0, 0, 0" "1.000000,1.000000,1.000000") false)))
      ;[0 0.6304 1] Handle Left wall height
      (for _index_11 (range 0 (- (Variables|Default|GetWallTileX) 1))
        ;[0 0.5139 1] Entry check
        (if (or (Variables|Default|GetIsOriginRoom) (!= _index_11 0))
          (if (Variables|Default|GetManualDoors)
            (CallFunction|ManualDoorL (== (Math|Integer|%(Integer) _index_11 (Variables|Default|GetDoorEvery)) (Variables|Default|GetDoorRemainder)) (Math|Vector|MakeVector 0.0 0.0 (* _index_11 (Variables|Default|GetWallSizeX))) "0.000000,90.000000,0.000000")
            (else
              (CallFunction|WallorDoorL (== (Math|Integer|%(Integer) _index_11 (Variables|Default|GetDoorEvery)) (Variables|Default|GetDoorRemainder)) (Math|Vector|MakeVector 0.0 0.0 (* _index_11 (Variables|Default|GetWallSizeX))) "0.000000,90.000000,0.000000")))))
      (Variables|Default|SetInstancedDoorsL 0)
      ;[0 0.6006 1] Handle Right wall Height
      (for _index_12 (range 0 (- (Variables|Default|GetWallTileX) 1))
        (if (Variables|Default|GetManualDoors)
          (CallFunction|ManualDoorR (== (Math|Integer|%(Integer) _index_12 (Variables|Default|GetManualRightDoorEvery)) (Variables|Default|GetManualRightDoorDisplacer)) (Math|Vector|MakeVector (* (Variables|Default|GetRoomTilesX) _tilesizex) _tilesizex (* _index_12 _tilesizex)) "0.000000,-90.000000,0.000000")
          (else
            (CallFunction|WallorDoorR (== (Math|Integer|%(Integer) _index_12 (Variables|Default|GetDoorEvery)) (Variables|Default|GetDoorRemainder)) (Math|Vector|MakeVector (* (Variables|Default|GetRoomTilesX) _tilesizex) _tilesizex (* _index_12 _tilesizex)) "0.000000,-90.000000,0.000000" false))))
      (Variables|Default|SetInstancedDoorsR 0)
      ;[0 0.4099 1] Set bound box
      (if (Variables|Default|GetHasBounds)
        (Collision|SetCollisionEnabled (Variables|Default|GetBox) "QueryAndPhysics")
        (else
          (Collision|SetCollisionEnabled (Variables|Default|GetBox) "NoCollision"))))))

(fn WallorDoorR
  (params (CanDoor :type Boolean) (InstanceTransformLocation :type Vector) (InstanceTransformRotation :type Rotator) (IsLeftDoor :type Boolean))
  (bind _returnvalue (Transformation|GetActorTransform))
  (bind _rightdoorcount (Variables|Default|GetRightDoorCount))
  (bind _returnvalue_2 (Math|Transform|TransformLocation _returnvalue InstanceTransformLocation))
  (bind _returnvalue_3 (Math|Transform|TransformRotation _returnvalue InstanceTransformRotation))
  ;[0 0.5622 1] Is this a door
  (if (and CanDoor (Class|KismetMathLibrary|RandomBoolwithWeightfromStream (Variables|Default|GetRoomStream) (/ (- _rightdoorcount (Utilities|Array|Length (Variables|Default|GetDoors))) _rightdoorcount)))
    ;[0 0.4894 1] Transform location and rotation to world space, spawn door and add to array
    (bind _returnvalue_4 (Game|SpawnActorfromClass "/Game/_Renato/Procedural/SpawnedObjects/BP_Doors.BP_Doors_C" (Math|Transform|MakeTransform _returnvalue_2 _returnvalue_3 "1.000000,1.000000,1.000000") "Undefined" "MultiplyWithRoot" 0 true 0))
    (Utilities|Array|Add (Variables|Default|GetDoors) _returnvalue_4)
    (Utilities|Array|SetArrayElem (Variables|/Script/Engine.Actor|GetTags _returnvalue_4) 0 "InstancedDoor")
    (else
      ;[0 0.5514 1] Add wall instead
      (bind _returnvalue_5 (Components|InstancedStaticMesh|AddInstance (Variables|Default|GetIndexedWall) (Math|Transform|MakeTransform InstanceTransformLocation InstanceTransformRotation "1.000000,1.000000,1.000000") false))
      ;[0 0.4466 1] Add colliders to walls
      (bind _returnvalue_6 (Game|SpawnActorfromClass "/Game/_Renato/Procedural/BP_WallCollision.BP_WallCollision_C" (Math|Transform|MakeTransform _returnvalue_2 _returnvalue_3 "1.000000,1.000000,1.000000") "Undefined" "MultiplyWithRoot" 0 _returnvalue_5 0))
      (Utilities|Array|Add (Variables|Default|GetWallCollisions) _returnvalue_6))))

(fn ManualDoorR
  (params (CanDoor :type Boolean) (InstancedTransformLocation :type Vector) (InstancedTransformRotaiton :type Rotator))
  (bind _returnvalue (Transformation|GetActorTransform))
  (bind _returnvalue_2 (Transformation|GetActorTransform))
  (bind _returnvalue_3 (Transformation|GetActorTransform))
  (bind _rightdoorcount (Variables|Default|GetRightDoorCount))
  (if (and CanDoor (and (> _rightdoorcount 0) (<= (Variables|Default|GetInstancedDoorsR) _rightdoorcount)))
    (if (not (Variables|Default|GetNoDoor))
      (if (Variables|Default|GetLockedDoor)
        (Game|SpawnActorfromClass "/Game/_Renato/LockedDoor/BP_LockedDoor.BP_LockedDoor_C" (Math|Transform|MakeTransform (Math|Transform|TransformLocation _returnvalue_2 InstancedTransformLocation) (Math|Transform|TransformRotation _returnvalue_2 InstancedTransformRotaiton) "1.000000,1.000000,1.000000") "Undefined" "MultiplyWithRoot" 0 0)
        (else
          ;[0 0.4894 1] Transform location and rotation to world space, spawn door and add to array
          (bind _returnvalue_4 (Game|SpawnActorfromClass "/Game/_Renato/Procedural/SpawnedObjects/BP_Doors.BP_Doors_C" (Math|Transform|MakeTransform (Math|Transform|TransformLocation _returnvalue InstancedTransformLocation) (Math|Transform|TransformRotation _returnvalue InstancedTransformRotaiton) "1.000000,1.000000,1.000000") "Undefined" "MultiplyWithRoot" 0 true 0))
          (Utilities|Array|Add (Variables|Default|GetDoors) _returnvalue_4)
          (Utilities|Array|SetArrayElem (Variables|/Script/Engine.Actor|GetTags _returnvalue_4) 0 "InstancedDoor")
          (Math|Integer|IncrementInt (Variables|Default|GetInstancedDoorsR)))))
    (else
      (bind _returnvalue_5 (Components|InstancedStaticMesh|AddInstance (Variables|Default|GetIndexedWall) (Math|Transform|MakeTransform InstancedTransformLocation InstancedTransformRotaiton "1.000000,1.000000,1.000000") false))
      (bind _returnvalue_6 (Game|SpawnActorfromClass "/Game/_Renato/Procedural/BP_WallCollision.BP_WallCollision_C" (Math|Transform|MakeTransform (Math|Transform|TransformLocation _returnvalue_3 InstancedTransformLocation) (Math|Transform|TransformRotation _returnvalue_3 InstancedTransformRotaiton) "1.000000,1.000000,1.000000") "Undefined" "MultiplyWithRoot" 0 _returnvalue_5 0))
      (Utilities|Array|Add (Variables|Default|GetWallCollisions) _returnvalue_6))))

(fn ManualDoorL
  (params (CanDoor :type Boolean) (Instance%20Transform%20Location :type Vector) (InstanceTransformRotation :type Rotator))
  (bind _returnvalue (Transformation|GetActorTransform))
  (bind _leftdoorcount (Variables|Default|GetLeftDoorCount))
  (bind _returnvalue_2 (Math|Transform|TransformLocation _returnvalue Instance%20Transform%20Location))
  (bind _returnvalue_3 (Math|Transform|TransformRotation _returnvalue InstanceTransformRotation))
  (if (and CanDoor (and (> _leftdoorcount 0) (<= (Variables|Default|GetInstancedDoorsL) _leftdoorcount)))
    (if (not (Variables|Default|GetNoDoor))
      ;[0 0.4894 1] Transform location and rotation to world space, spawn door and add to array
      (bind _returnvalue_4 (Game|SpawnActorfromClass "/Game/_Renato/Procedural/SpawnedObjects/BP_Doors.BP_Doors_C" (Math|Transform|MakeTransform _returnvalue_2 _returnvalue_3 "1.000000,1.000000,1.000000") "Undefined" "MultiplyWithRoot" 0 true 0))
      (Utilities|Array|Add (Variables|Default|GetDoors) _returnvalue_4)
      (Utilities|Array|SetArrayElem (Variables|/Script/Engine.Actor|GetTags _returnvalue_4) 0 "InstancedDoor")
      (Math|Integer|IncrementInt (Variables|Default|GetInstancedDoorsL)))
    (else
      (bind _returnvalue_5 (Components|InstancedStaticMesh|AddInstance (Variables|Default|GetIndexedWall) (Math|Transform|MakeTransform Instance%20Transform%20Location InstanceTransformRotation "1.000000,1.000000,1.000000") false))
      (bind _returnvalue_6 (Game|SpawnActorfromClass "/Game/_Renato/Procedural/BP_WallCollision.BP_WallCollision_C" (Math|Transform|MakeTransform _returnvalue_2 _returnvalue_3 "1.000000,1.000000,1.000000") "Undefined" "MultiplyWithRoot" 0 _returnvalue_5 0))
      (Utilities|Array|Add (Variables|Default|GetWallCollisions) _returnvalue_6))))