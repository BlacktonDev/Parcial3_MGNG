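; BP_WallCollision is a procedural wall marker actor that carries an index identifying a wall in the procedural room.
; On BeginPlay and on Update it stores the index and shows it on a DebugIndex text.
; RemoveIndex finds BP_ProceduralRoom actors, calls DeleteWall with its index, then destroys itself.
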(event Custom|Update
  (params (NewIndex :type Integer))
  (bind _output_get (Variables|Default|SetIndex NewIndex))
  (Rendering|Components|TextRender|SetText (Variables|Default|GetDebugIndex) (Utilities|Text|ToText(Integer) _output_get)))

(event Custom|RemoveIndex
  (bind _outactors (Actor|GetAllActorsOfClass "/Game/_Renato/Procedural/BP_ProceduralRoom.BP_ProceduralRoom_C"))
  (Default|DeleteWall _outactors (Variables|Default|GetIndex))
  (Actor|DestroyActor))

(event EventBeginPlay
  (CallFunction|Update (Variables|Default|GetIndex)))

(fn ConstructionScript)