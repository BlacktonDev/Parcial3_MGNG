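; BP_CameraManager is an actor that smoothly follows a target's position, serving as a follow camera rig.
; Every Tick, UpdateCameraPos moves the actor with VInterpTo toward FollowTarget's location, with CameraDelay as the interpolation speed.
; LockX and LockHeight optionally hold the X and Z axes at their current values, while Y always follows the target.
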(event EventBeginPlay)

(event Collision|EventActorBeginOverlap
  (params (OtherActor :type Actor%20Object%20Reference)))

(event EventTick
  (params (DeltaSeconds :type Float%20%28single-precision%29))
  (CallFunction|UpdateCameraPos))

(fn ConstructionScript)

(fn UpdateCameraPos
  (bind _returnvalue (Transformation|GetActorLocation))
  (bind _followtarget (Variables|Default|GetFollowTarget))
  (bind _returnvalue_2 (Transformation|GetActorLocation _followtarget))
  (Transformation|SetActorLocation (Math|Interpolation|VInterpTo (Transformation|GetActorLocation) (Math|Vector|MakeVector (select (Variables|Default|GetLockX) (.x _returnvalue) (.x _returnvalue_2)) (.y _returnvalue_2) (select (Variables|Default|GetLockHeight?) (.z _returnvalue) (.z _returnvalue_2))) (Utilities|Time|GetWorldDeltaSeconds) (Variables|Default|GetCameraDelay)) false false))