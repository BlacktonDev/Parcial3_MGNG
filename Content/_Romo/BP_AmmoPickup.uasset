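; BP_AmmoPickup is a collectible that gives the player one round of ammo when touched.
; On sphere overlap it casts to BP_Player and proceeds only if current ammo is not already at maximum.
; It increments ammo clamped to the max, calls GetAmmo on the player's UI widget, then destroys itself, so a full player leaves the pickup in place.
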(event OnComponentBeginOverlap(Sphere)
  (params (OverlappedComponent :type Primitive%20Component%20Object%20Reference) (OtherActor :type Actor%20Object%20Reference) (OtherComp :type Primitive%20Component%20Object%20Reference) (OtherBodyIndex :type Integer) (bFromSweep :type Boolean) (SweepResult :type Hit%20Result%20Structure%20%28by%20ref%29))
  (bind _asbp_player (Utilities|Casting|CastToBP_Player OtherActor))
  (bind _output_get (Variables|Default|SetBP%20Player%20Reference _asbp_player))
  (if (not (== (Variables|/Game/_Romo/Character/BP_Player.BP_Player_C|GetCurrentAmmo _output_get) (Variables|/Game/_Romo/Character/BP_Player.BP_Player_C|GetMaxAmmo _output_get)))
    (Variables|/Game/_Romo/Character/BP_Player.BP_Player_C|SetCurrentAmmo (Variables|Default|GetBP%20Player%20Reference) (Math|Integer|Clamp(Integer) (+ (Variables|/Game/_Romo/Character/BP_Player.BP_Player_C|GetCurrentAmmo (Variables|Default|GetBP%20Player%20Reference)) 1) 1 (Variables|/Game/_Romo/Character/BP_Player.BP_Player_C|GetMaxAmmo (Variables|Default|GetBP%20Player%20Reference))))
    (Default|GetAmmo (Variables|/Game/_Romo/Character/BP_Player.BP_Player_C|GetPlayerUIWidget (Variables|Default|GetBP%20Player%20Reference)))
    (Actor|DestroyActor)))

(event EventBeginPlay)

(event Collision|EventActorBeginOverlap
  (params (OtherActor :type Actor%20Object%20Reference)))

(event EventTick
  (params (DeltaSeconds :type Float%20%28single-precision%29)))

(fn ConstructionScript)