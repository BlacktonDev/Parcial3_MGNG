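; BP_HealthPickup is a pickup that heals the player when they touch it.
; A sphere overlap casts the other actor to BP_Player and continues only if health is not already at maximum.
; It adds HealingAmount, clamped to MaxHealth, shows a healing message through the player's UI widget, then destroys itself.
; At full health the pickup stays in the world.
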(event OnComponentBeginOverlap(Sphere)
  (params (OverlappedComponent :type Primitive%20Component%20Object%20Reference) (OtherActor :type Actor%20Object%20Reference) (OtherComp :type Primitive%20Component%20Object%20Reference) (OtherBodyIndex :type Integer) (bFromSweep :type Boolean) (SweepResult :type Hit%20Result%20Structure%20%28by%20ref%29))
  (bind _asbp_player (Utilities|Casting|CastToBP_Player OtherActor))
  (Variables|Default|SetBP%20Player%20Reference _asbp_player)
  (if (not (== (Variables|/Game/_Romo/Character/BP_Player.BP_Player_C|GetMaxHealth (Variables|Default|GetBP%20Player%20Reference)) (Variables|/Game/_Romo/Character/BP_Player.BP_Player_C|GetCurrentHealth (Variables|Default|GetBP%20Player%20Reference))))
    (Variables|/Game/_Romo/Character/BP_Player.BP_Player_C|SetCurrentHealth (Variables|Default|GetBP%20Player%20Reference) (Math|Float|Clamp(Float) (+ (Variables|/Game/_Romo/Character/BP_Player.BP_Player_C|GetCurrentHealth (Variables|Default|GetBP%20Player%20Reference)) (Variables|Default|GetHealingAmount)) 1.0 (Variables|/Game/_Romo/Character/BP_Player.BP_Player_C|GetMaxHealth (Variables|Default|GetBP%20Player%20Reference))))
    (Class|BPIHealthWidget|UpdateDamage(Message) (Variables|/Game/_Romo/Character/BP_Player.BP_Player_C|GetPlayerUIWidget (Variables|Default|GetBP%20Player%20Reference)) (Utilities|Text|ToText(Float) (Variables|Default|GetHealingAmount) "HalfToEven") true)
    (Actor|DestroyActor)))

(event EventBeginPlay)

(event Collision|EventActorBeginOverlap
  (params (OtherActor :type Actor%20Object%20Reference)))

(event EventTick
  (params (DeltaSeconds :type Float%20%28single-precision%29)))

(fn ConstructionScript)