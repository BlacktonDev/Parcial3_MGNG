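; BP_PlayerProjectile is the player's projectile actor, which damages enemies and destroys other projectiles on contact.
; On a Sphere1 hit it enables gravity on its ProjectileMovement, then checks the other actor's tags.
; Actors tagged "enemy" receive damage and actors tagged "projectile" are destroyed.
; The projectile then destroys itself, after a delay when it hit anything else.
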(event OnComponentBeginOverlap(Sphere1)
  (params (OverlappedComponent :type Primitive%20Component%20Object%20Reference) (OtherActor :type Actor%20Object%20Reference) (OtherComp :type Primitive%20Component%20Object%20Reference) (OtherBodyIndex :type Integer) (bFromSweep :type Boolean) (SweepResult :type Hit%20Result%20Structure%20%28by%20ref%29)))

(event OnComponentHit(Sphere1)
  (params (HitComponent :type Primitive%20Component%20Object%20Reference) (OtherActor :type Actor%20Object%20Reference) (OtherComp :type Primitive%20Component%20Object%20Reference) (NormalImpulse :type Vector :default "0, 0, 0") (Hit :type Hit%20Result%20Structure%20%28by%20ref%29))
  (Variables|/Script/Engine.ProjectileMovementComponent|SetProjectileGravityScale (Variables|Default|GetProjectileMovement) 1.0)
  (if (Actor|ActorHasTag OtherActor "enemy")
    (Game|Damage|ApplyDamage OtherActor (Variables|Default|GetBase%20Damage) 0 self)
    (elif (Actor|ActorHasTag OtherActor "projectile")
      (Actor|DestroyActor OtherActor)
      (else
        (Utilities|FlowControl|Delay (Variables|Default|GetDuration)))))
  (Actor|DestroyActor))

(event EventBeginPlay)

(event Collision|EventActorBeginOverlap
  (params (OtherActor :type Actor%20Object%20Reference)))

(event EventTick
  (params (DeltaSeconds :type Float%20%28single-precision%29)))

(fn ConstructionScript)